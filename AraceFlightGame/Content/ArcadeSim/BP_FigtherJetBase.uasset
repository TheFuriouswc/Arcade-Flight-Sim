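; Base arcade fighter jet pawn that taxis on the ground, takes off, flies and lands under Enhanced Input control.
; A Flying flag switches inputs between ground roll with free camera look and throttle with pitch and yaw of the jet.
; Tick moves the airborne jet along its forward vector, scales exhaust with speed and line-traces downward to land at low throttle.
; Input also sets wheel, aileron and rudder rotation variables.
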(event `self.ReceiveBeginPlay`
  ;[0 0 0] Event BeginPlay
  (bind _asplayer_controller (cast `PlayerController` (`self.GetController`)))
  (bind _returnvalue (pcsubsystem `EnhancedInputLocalPlayerSubsystem` _asplayer_controller))
  (`/Engine/EditorBlueprintResources/StandardMacros.IsValid` _returnvalue
    (:`Is Valid`
      (`EnhancedInputSubsystemInterface.AddMappingContext` _returnvalue "/Game/ArcadeSim/Inputs/Default_IMC.Default_IMC" 0 (struct))
      (`|ExecutionSequence`
        (:`then_0`
          ;;[1 1 1] When Plane Take Off, It Should Fly At The Minimum Set Speed
          (set `self.TargetThrusterSpeed` (`self.MaximumThrusterSpeed`))
          ;;[1 1 1] Setting offset for landing trace
          (set `self.Star Z Offset` (`self.Plane Z Offset`)))
        (:`then_1`
          ;;[1 1 1] Set Scale of exhaust particles to 0 as it should become more intense with speed
          (`SceneComponent.SetRelativeScale3D` (`self.LeftExhaust`) (0.0 0.0 0.0))
          (`SceneComponent.SetRelativeScale3D` (`self.RightExhaust`) (0.0 0.0 0.0)))))))

(event `self.ReceiveTick`
  (params (DeltaSeconds :type "Float (single-precision)"))
  (bind _leftexhaust (`self.LeftExhaust`))
  (bind _returnvalue (`KismetMathLibrary.NormalizeToRange` (`self.CurrentThrusterSpeed`) 0.0 (`self.MaximumThrusterSpeed`)))
  ;[0 0 0] Event Tick
  (`|ExecutionSequence`
    (:`then_0`
      ;;[1 1 1] For Grounded Movement. Intrep value set to low value as jet should speed up very gradually when on ground
      (bind _output_get (set `self.MoveForwardInterp` (`KismetMathLibrary.FClamp` (`KismetMathLibrary.FInterpTo` (stale _output_get) (`|GetInputActionValue`) (`GameplayStatics.GetWorldDeltaSeconds`) 0.2))))
      ;[1 1 1] Set exhaust particle scale relative to speed. 0 If not flying but interp speed is low so if landing it while take a while for the aprticles fade to zero scale
      (`SceneComponent.SetRelativeScale3D` _leftexhaust (`KismetMathLibrary.VInterpTo` (`SceneComponent.RelativeScale3D` _leftexhaust) (`KismetMathLibrary.SelectVector` (`KismetMathLibrary.MakeVector` _returnvalue _returnvalue _returnvalue) (0.0 0.0 0.0) (`self.Flying?`)) (`GameplayStatics.GetWorldDeltaSeconds`) (`KismetMathLibrary.SelectFloat` 4.0 0.5 (`self.Flying?`))))
      (`SceneComponent.SetRelativeScale3D` (`self.RightExhaust`) (`KismetMathLibrary.VInterpTo` (`SceneComponent.RelativeScale3D` _leftexhaust) (`KismetMathLibrary.SelectVector` (`KismetMathLibrary.MakeVector` _returnvalue _returnvalue _returnvalue) (0.0 0.0 0.0) (`self.Flying?`)) (`GameplayStatics.GetWorldDeltaSeconds`) (`KismetMathLibrary.SelectFloat` 4.0 0.5 (`self.Flying?`)))))
    (:`then_1`
      ;;[1 1 1] Is Flying
      (if (`self.Flying?`)
        (`self.Add Flight Movement`)
        (`self.Landing Trace` "ForOneFrame" (`self.Star Z Offset`))))))

(event `EnhancedInput|/Game/ArcadeSim/Inputs/Actions/IA_MoveForward`
  (params (ActionValue :type "Float (double-precision)") (ElapsedSeconds :type "Float (double-precision)") (TriggeredSeconds :type "Float (double-precision)") (InputAction :type "InputAction Object Reference" :default "/Game/ArcadeSim/Inputs/Actions/IA_MoveForward.IA_MoveForward"))
  (bind _returnvalue (`GameplayStatics.GetPlayerController` 0))
  (bind _wheelrotationsidemax (`self.WheelRotationSideMax`))
  (bind (_wheelrotation_roll _wheelrotation_pitch _wheelrotation_yaw) (`KismetMathLibrary.BreakRotator` (`self.WheelRotation`)))
  (bind (_returnvalue_roll _returnvalue_pitch) (`KismetMathLibrary.BreakRotator` (`SceneComponent.GetSocketRotation` (`self.SK_West_Fighter_F15E`) "front_wheel_1_jnt")))
  ;[0 1 0.9575] Move Forward
  ;;[1 1 1] If fly, then move forward inputs should increase/decrease flight speed. If not then it will add movement on floor using offset
  (:`Triggered`
    (if (`self.Flying?`)
      (set `self.TargetThrusterSpeed` (`KismetMathLibrary.FClamp` (+ (* ActionValue (`GameplayStatics.GetWorldDeltaSeconds`) 2500.0) (`self.TargetThrusterSpeed`)) (`self.MininumThrusterSpeed`) (`self.MaximumThrusterSpeed`))))
    (if (not (`self.Flying?`))
      (`|ExecutionSequence`
        (:`then_0`
          ;;[1 1 1] Slowly move plane across ground, with speed getting higher the longer move forward is held down. Z is zero=ed out since it should not move up and only on same plane
          (`self.K2_AddActorWorldOffset` (`KismetMathLibrary.MakeVector` (.x (* (`self.GetActorForwardVector`) (`self.MoveForwardInterp`) (/ (`self.TargetThrusterSpeed`) 500.0))) (.y (* (`self.GetActorForwardVector`) (`self.MoveForwardInterp`) (/ (`self.TargetThrusterSpeed`) 500.0)))))
          ;;[1 1 1] If Moving fast enough on ground and space is pressed, the plane will go into flying mode. Lag is turned on for sping arm for smother fly controlls and small offset added to prevent crashing on ground immediately upon take off
          (if (and (> (`self.MoveForwardInterp`) 0.7) (or (`PlayerController.IsInputKeyDown` _returnvalue "G") (`PlayerController.IsInputKeyDown` _returnvalue "Gamepad_LeftThumbstick")))
            (set `self.Flying?` true)
            (bind _output_get (set `SpringArmComponent.bUsePawnControlRotation` false (`self.SpringArm`)))
            (set `CameraComponent.bUsePawnControlRotation` _output_get (`self.Camera`))
            (`self.K2_AddActorWorldOffset` (0.0 0.0 25.0))))
        (:`then_1`
          ;;[1 1 1] Setting Wheel Rotation for side and forward directions
          (set `self.WheelRotation` (`KismetMathLibrary.MakeRotator` 0.0 (+ _returnvalue_pitch (* (`self.MoveForwardInterp`) -500.0)) (`KismetMathLibrary.FInterpTo` _wheelrotation_yaw (`KismetMathLibrary.MapRangeClamped` (`|GetInputActionValue`) -1.0 1.0 (* _wheelrotationsidemax -1.0) _wheelrotationsidemax) (`GameplayStatics.GetWorldDeltaSeconds`) 0.4))))))))

(event `EnhancedInput|/Game/ArcadeSim/Inputs/Actions/IA_LookUp`
  (params (ActionValue :type "Float (double-precision)") (ElapsedSeconds :type "Float (double-precision)") (TriggeredSeconds :type "Float (double-precision)") (InputAction :type "InputAction Object Reference" :default "/Game/ArcadeSim/Inputs/Actions/IA_LookUp.IA_LookUp"))
  (bind _returnvalue (`GameplayStatics.GetWorldDeltaSeconds`))
  (bind _alilionexteriorrotationsmax (`self.AlilionExteriorRotationsMax`))
  (bind _alilioninteriorrotationsmax (`self.AlilionInteriorRotationsMax`))
  (bind _returnvalue_2 (* ActionValue (`KismetMathLibrary.SelectFloat` -1.0 1.0 (`self.InvertVerticalFlight?`))))
  ;[0 1 0.9575] Look up input. If not flying add camera rotation. If not then add rotation to plane and since spring arm is attached it will automatcally adjust camera behind plane
  (:`Triggered`
    (if (`self.Flying?`)
      (bind _output_get (set `self.FlightPitch` (`KismetMathLibrary.FInterpTo` (stale _output_get) _returnvalue_2 _returnvalue 10.0)))
      (`self.K2_AddActorLocalRotation` (`KismetMathLibrary.MakeRotator` 0.0 (* _output_get _returnvalue (`self.FlightTurnRate`))))
      (set `self.AlilionInteriorRotations` (`KismetMathLibrary.MakeRotator` 0.0 (`KismetMathLibrary.MapRangeClamped` (`self.FlightPitch`) -1.0 1.0 _alilioninteriorrotationsmax (* _alilioninteriorrotationsmax -1.0))))
      (set `self.AlilionExteriorRotations` (`KismetMathLibrary.MakeRotator` 0.0 (`KismetMathLibrary.MapRangeClamped` (`self.FlightPitch`) -1.0 1.0 _alilionexteriorrotationsmax (* _alilionexteriorrotationsmax -1.0))))
      (else
        (`self.AddControllerPitchInput` _returnvalue_2)))))

(event `EnhancedInput|/Game/ArcadeSim/Inputs/Actions/IA_TurnRight`
  (params (ActionValue :type "Float (double-precision)") (ElapsedSeconds :type "Float (double-precision)") (TriggeredSeconds :type "Float (double-precision)") (InputAction :type "InputAction Object Reference" :default "/Game/ArcadeSim/Inputs/Actions/IA_TurnRight.IA_TurnRight"))
  (bind _returnvalue (`GameplayStatics.GetWorldDeltaSeconds`))
  (bind _rudderrotationmax (`self.RudderRotationMax`))
  ;[0 1 0.9575] Look up input. If not flying add camera rotation. If not then add rotation to plane and since spring arm is attached it will automatcally adjust camera behind plane
  (:`Triggered`
    (if (`self.Flying?`)
      (bind _output_get (set `self.FlightTurn` (`KismetMathLibrary.FInterpTo` (stale _output_get) ActionValue _returnvalue 10.0)))
      (`self.K2_AddActorLocalRotation` (`KismetMathLibrary.MakeRotator` 0.0 0.0 (* _output_get _returnvalue (`self.FlightTurnRate`))))
      (set `self.BackRudderRotation` (`KismetMathLibrary.MakeRotator` 0.0 0.0 (`KismetMathLibrary.MapRangeClamped` (`self.FlightTurn`) -1.0 1.0 _rudderrotationmax (* _rudderrotationmax -1.0))))
      (else
        (`self.AddControllerYawInput` ActionValue)))))

(fn `Add Flight Movement`
  (bind _returnvalue (`GameplayStatics.GetWorldDeltaSeconds`))
  ;[1 1 1] Set flight Speed
  (bind _output_get (set `self.CurrentThrusterSpeed` (`KismetMathLibrary.FInterpTo` (stale _output_get) (`self.TargetThrusterSpeed`) _returnvalue 8.0)))
  ;[1 1 1] Add movement in forward direction to plane
  (`self.K2_AddActorWorldOffset` (* (`SceneComponent.GetForwardVector` (`self.SK_West_Fighter_F15E`)) (* _output_get _returnvalue)) true))

(fn `Landing Trace`
  (params (Debug :type "EDrawDebugTrace Enum" :default "None") (`Spawned Z Offset` :type "Float (double-precision)"))
  (bind _returnvalue (`self.K2_GetActorLocation`))
  (bind (_returnvalue_roll _returnvalue_pitch _returnvalue_yaw) (`KismetMathLibrary.BreakRotator` (`self.K2_GetActorRotation`)))
  ;[1 1 1] Do line trace from plane center to postion under the wheel
  (bind (_outhit _returnvalue_2) (`KismetSystemLibrary.LineTraceSingle` _returnvalue (- _returnvalue (`KismetMathLibrary.MakeVector` 0.0 0.0 `Spawned Z Offset`)) "TraceTypeQuery1" false (`|MakeArray` self :!type "Actor Object Reference") Debug))
  ;[1 1 1] Can only land if speed is low enough(controlled by holding move forward or backward)
  (if _returnvalue_2
    (if (< (`KismetMathLibrary.MapRangeClamped` (`self.TargetThrusterSpeed`) (`self.MininumThrusterSpeed`) (`self.MaximumThrusterSpeed`) 0.0 1.0) 0.5)
      ;[1 1 1] Align plane with floor(using custom variables instead of normals). Rotation is only retained a yaw. Location include of wheels offset
      (set `self.Flying?` false)
      (`self.K2_SetActorRelativeTransform` (`KismetMathLibrary.MakeTransform` (`KismetMathLibrary.VInterpTo` (`self.K2_GetActorLocation`) (+ (`.TraceEnd` (`GameplayStatics.BreakHitResult` _outhit)) (`KismetMathLibrary.MakeVector` 0.0 0.0 (`local.Spawned Z Offset`))) (`GameplayStatics.GetWorldDeltaSeconds`) 3.0) (`KismetMathLibrary.MakeRotator` 0.0 0.0 _returnvalue_yaw)))
      ;[1 1 1] Set variables
      (set `SpringArmComponent.bUsePawnControlRotation` true (`self.SpringArm`))
      (set `self.MoveForwardInterp` 1.0))))

(fn `Set Camera Lag`
  (bind _springarm (`self.SpringArm`))
  (bind _returnvalue (`KismetMathLibrary.SelectFloat` 10.0 1000.0 (`self.Flying?`)))
  ;[1 1 1] If not flying the lag should be hign enough to not be recongnisable since it is still recuired for smooth camera return when landing
  (set `SpringArmComponent.CameraLagSpeed` _returnvalue _springarm)
  (set `SpringArmComponent.CameraLagSpeed` _returnvalue _springarm))

(fn `UserConstructionScript`)