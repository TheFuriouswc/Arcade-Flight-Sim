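; BP_MissleBase is a base missile actor that stays still until fired, then launches toward a homing target.
; BeginPlay stops the ProjectileMovement component immediately.
; FireAway passes HomingTargetComponent and Speed (as InitialSpeed) to ProjectileMovement, then sets Velocity to the actor's unscaled forward vector.
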(event `self.ReceiveBeginPlay`
  (`MovementComponent.StopMovementImmediately` (`self.ProjectileMovement`)))

(event `FireAway`
  (bind _projectilemovement (`self.ProjectileMovement`))
  (set `ProjectileMovementComponent.HomingTargetComponent` (`self.Homing Target Component`) (`self.ProjectileMovement`))
  (set `ProjectileMovementComponent.InitialSpeed` (`self.Speed`) _projectilemovement)
  (set `MovementComponent.Velocity` (`self.GetActorForwardVector`) _projectilemovement))

(fn `UserConstructionScript`)