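; BP_BulletMaster is a bullet projectile that flies toward an aim point and deals damage on hit.
; BeginPlay sets its velocity via a suggested toss toward AliginToCamera, adding PlayerSpeed to launch speed, and spawns a muzzle flash.
; Box hits branch on BlockActors, then fire a radial impulse, spawn impact particles, apply damage and destroy the bullet.
; The class-exclusion expression inside BlockActors is left unused.
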(event `self.ReceiveBeginPlay`
  ;[0 0 0] event beginplay
  (bind _tossvelocity (`GameplayStatics.BlueprintSuggestProjectileVelocity` (`self.K2_GetActorLocation`) (`self.AliginToCamera`) (+ (`self.PlayerSpeed`) (`ProjectileMovementComponent.InitialSpeed` (`self.ProjectileMovement`))) 0.0 "DoNotTrace"))
  (set `MovementComponent.Velocity` _tossvelocity (`self.ProjectileMovement`))
  (`GameplayStatics.SpawnEmitterAtLocation` "/Game/MilitaryWeapDark/FX/P_AssaultRifle_MuzzleFlash.P_AssaultRifle_MuzzleFlash"))

(event `self.Box.OnComponentHit`
  (params (HitComponent :type "PrimitiveComponent Object Reference") (OtherActor :type "Actor Object Reference") (OtherComp :type "PrimitiveComponent Object Reference") (NormalImpulse :type "Vector Structure") (Hit :type "HitResult Structure (by ref)"))
  (if (or (!= (`GameplayStatics.GetObjectClass` HitComponent) "/Game/ArcadeSim/Blueprints/Jets/BP_FigtherJetBase.BP_FigtherJetBase_C") (!= (`GameplayStatics.GetObjectClass` HitComponent) "/Game/ArcadeSim/Blueprints/Weapons/BP_MissleBase.BP_MissleBase_C") (!= (`GameplayStatics.GetObjectClass` HitComponent) "BP_BulletMaster_C"))
    (`RadialForceComponent.FireImpulse` (`self.RadialForce`))
    (`GameplayStatics.SpawnEmitterAtLocation` "/Game/MilitaryWeapDark/FX/P_Impact_Metal_Small_01.P_Impact_Metal_Small_01" (`.Location` (`GameplayStatics.BreakHitResult` Hit)))
    (`GameplayStatics.ApplyDamage` OtherActor 1.0)
    (`self.K2_DestroyActor`)))

(fn `UserConstructionScript`)