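; Enemy homing missile that, once fired, starts its Niagara effect and steers ProjectileMovement toward its assigned target component.
; A countermeasure overlap sphere switches homing to any detected BP_Flare, while a hit detector applies damage, spawns explosion effects and destroys the missile.
; A Tick-driven delay expires it after fifteen seconds.
; Expiry and hits on anything other than BP_FigtherJetBase attempt a random, subtitled missile-evaded voice line at the player.
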(event `self.ReceiveTick`
  (params (DeltaSeconds :type "Float (single-precision)"))
  (bind _returnvalue (`KismetMathLibrary.RandomIntegerInRange` 1 3))
  (`KismetSystemLibrary.Delay` 15.0)
  (if (== _returnvalue 1.0)
    (`self.SpawnSubtitles` "/Game/ArcadeSim/SoundEffects/Voicelines/Player/Missle_Evaded.Missle_Evaded" "/Game/ArcadeSim/Subtitles/Player/DTSub_PlayerDefeated1.DTSub_PlayerDefeated1")
    (`self.K2_DestroyActor` :!label _label)
    (elif (== _returnvalue 2.0)
      (`self.SpawnSubtitles` "/Game/ArcadeSim/SoundEffects/Voicelines/Player/missleevadedthxgod.missleevadedthxgod" "/Game/ArcadeSim/Subtitles/Player/DTSub_PlayerDefeated2.DTSub_PlayerDefeated2")
      (goto _label)
      (elif (== _returnvalue 3.0)
        (`self.SpawnSubtitles` "/Game/ArcadeSim/SoundEffects/Voicelines/Player/alimony.alimony" "/Game/ArcadeSim/Subtitles/Player/DTSub_PlayerDefeated3.DTSub_PlayerDefeated3")
        (goto _label)))))

(event `Fireaway`
  (bind _homing_target_component (`self.Homing Target Component`))
  (set `self.FireAway?` true)
  (`KismetSystemLibrary.Delay` 0.2)
  (`NiagaraComponent.SetAsset` (`self.Niagara`) "/Game/VigilanteContent/Projectiles/West_Missile_AIM120/FX/NS_West_Missile_AIM120.NS_West_Missile_AIM120" true)
  (set `ProjectileMovementComponent.HomingTargetComponent` _homing_target_component (`self.ProjectileMovement`))
  (`KismetSystemLibrary.Delay` 0.5)
  (`self.K2_SetActorRotation` (`KismetMathLibrary.FindLookAtRotation` (`self.K2_GetActorLocation`) (`SceneComponent.K2_GetComponentLocation` _homing_target_component))))

(event `self.BlueforDectector.OnComponentBeginOverlap`
  (params (OverlappedComponent :type "PrimitiveComponent Object Reference") (OtherActor :type "Actor Object Reference") (OtherComp :type "PrimitiveComponent Object Reference") (OtherBodyIndex :type Integer) (bFromSweep :type Boolean) (SweepResult :type "HitResult Structure (by ref)"))
  (bind _returnvalue (`KismetSystemLibrary.GetDisplayName` OtherActor))
  (bind _returnvalue_2 (`KismetMathLibrary.RandomIntegerInRange` 1 3))
  (if (and (or (!= (`GameplayStatics.GetObjectClass` OtherActor) "BP_EnemyMissle_C") (!= (`GameplayStatics.GetObjectClass` OtherActor) "/Game/ArcadeSim/Blueprints/Weapons/BP_MissleBase.BP_MissleBase_C") (!= (`GameplayStatics.GetObjectClass` OtherActor) "/Game/ArcadeSim/Blueprints/Weapons/BP_BulletMaster.BP_BulletMaster_C") (!= (`GameplayStatics.GetObjectClass` OtherActor) "/Game/ArcadeSim/Blueprints/Weapons/BP_BombMaster.BP_BombMaster_C") (!= (`GameplayStatics.GetObjectClass` OtherActor) "/Game/ArcadeSim/Blueprints/Enemy/BP_EnemySamBase.BP_EnemySamBase_C")) (`self.FireAway?`))
    (`GameplayStatics.ApplyDamage` OtherActor 25.0)
    (`NiagaraFunctionLibrary.SpawnSystemAtLocation` "/Game/ArcadeSim/VFX/Particles/FXS_BOOM.FXS_BOOM" (`self.K2_GetActorLocation`) (`self.K2_GetActorRotation`) (`self.GetActorScale3D`))
    (`GameplayStatics.PlaySoundAtLocation` "/Game/StarterContent/Audio/Explosion01.Explosion01" (`self.K2_GetActorLocation`) (struct) 1.0 1.0 0.0 null null null null)
    (set `self.FireAway?` false)
    (if (!= (`GameplayStatics.GetObjectClass` OtherActor) "/Game/ArcadeSim/Blueprints/Jets/BP_FigtherJetBase.BP_FigtherJetBase_C")
      (`KismetSystemLibrary.PrintString` _returnvalue)
      (if (== _returnvalue_2 1.0)
        (`self.SpawnSubtitles` "/Game/ArcadeSim/SoundEffects/Voicelines/Player/Missle_Evaded.Missle_Evaded" "/Game/ArcadeSim/Subtitles/Player/DTSub_PlayerDefeated1.DTSub_PlayerDefeated1")
        (`self.K2_DestroyActor` :!label _label_2)
        (elif (== _returnvalue_2 2.0)
          (`self.SpawnSubtitles` "/Game/ArcadeSim/SoundEffects/Voicelines/Player/missleevadedthxgod.missleevadedthxgod" "/Game/ArcadeSim/Subtitles/Player/DTSub_PlayerDefeated2.DTSub_PlayerDefeated2")
          (goto _label_2)
          (elif (== _returnvalue_2 3.0)
            (`self.SpawnSubtitles` "/Game/ArcadeSim/SoundEffects/Voicelines/Player/alimony.alimony" "/Game/ArcadeSim/Subtitles/Player/DTSub_PlayerDefeated3.DTSub_PlayerDefeated3")
            (goto _label_2))))
      (else
        (`KismetSystemLibrary.PrintString` _returnvalue)
        (`self.K2_DestroyActor`)))))

(event `self.CMDectector.OnComponentBeginOverlap`
  (params (OverlappedComponent :type "PrimitiveComponent Object Reference") (OtherActor :type "Actor Object Reference") (OtherComp :type "PrimitiveComponent Object Reference") (OtherBodyIndex :type Integer) (bFromSweep :type Boolean) (SweepResult :type "HitResult Structure (by ref)"))
  (bind _rootcomponent (`Actor.RootComponent` OtherActor))
  (if (and (or (!= (`GameplayStatics.GetObjectClass` OtherActor) "BP_EnemyMissle_C") (!= (`GameplayStatics.GetObjectClass` OtherActor) "/Game/ArcadeSim/Blueprints/Weapons/BP_MissleBase.BP_MissleBase_C") (!= (`GameplayStatics.GetObjectClass` OtherActor) "/Game/ArcadeSim/Blueprints/Weapons/BP_BulletMaster.BP_BulletMaster_C") (!= (`GameplayStatics.GetObjectClass` OtherActor) "/Game/ArcadeSim/Blueprints/Weapons/BP_BombMaster.BP_BombMaster_C") (!= (`GameplayStatics.GetObjectClass` OtherActor) "/Game/ArcadeSim/Blueprints/Enemy/BP_EnemySamBase.BP_EnemySamBase_C")) (`self.FireAway?`))
    (if (== (`GameplayStatics.GetObjectClass` OtherActor) "/Game/ArcadeSim/Blueprints/Weapons/BP_Flare.BP_Flare_C")
      (set `ProjectileMovementComponent.HomingTargetComponent` _rootcomponent (`self.ProjectileMovement`))
      (`KismetSystemLibrary.Delay` 0.5)
      (`self.K2_SetActorRotation` (`KismetMathLibrary.FindLookAtRotation` (`self.K2_GetActorLocation`) (`SceneComponent.K2_GetComponentLocation` _rootcomponent)))
      (`KismetSystemLibrary.PrintString` "Lock to flares"))))

(fn `UserConstructionScript`)