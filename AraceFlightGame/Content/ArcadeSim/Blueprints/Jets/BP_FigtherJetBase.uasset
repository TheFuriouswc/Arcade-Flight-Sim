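; Base pawn for an arcade fighter jet that taxis, takes off, flies and lands, with guns, switchable specials and lock-on.
; A Flying flag switches input between ground offsets with wheel animation and flight pitch, roll and thrust, moved by swept offsets each tick.
; A downward trace lands the jet at low speed.
; Timelines animate flaps and recenter the free-look camera, weapon inputs call dispatchers, and exhaust scales with speed.
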(event Custom|AililreonRotate
  (bind _alilioninteriorrotationsmax (Variables|MeshTransfroms|GetAlilionInteriorRotationsMax))
  (bind _alilioninteriorrotationsmax_2 (Variables|MeshTransfroms|GetAlilionInteriorRotationsMax))
  ;[0 1 0.9575] Move right input. if not flying then move on ground if moving forward as well. The if not then inputs will no rotate the plane
  ;;[1 1 1] Smoothly Rotate back Aililrons
  (if (!= (Variables|PlaneRotation|GetLastRotationAV) (Variables|PlaneRotation|GetRotateAV))
    (Variables|PlaneRotation|SetCurrentRotationAV (Variables|PlaneRotation|GetRotateAV))
    (bind _alpha (Timeline|AililonTimeline PlayFromStart)
      (:Update
        (Variables|MeshTransfroms|SetAlilionBackLeftRotations (Math|Rotator|MakeRotator 0.0 (Math|Float|Lerp (.pitch (Variables|MeshTransfroms|GetAlilionBackLeftRotations)) (Math|Float|MapRangeClamped (Input|EnhancedActionValues|GetIA_Rotate) -1.0 1.0 _alilioninteriorrotationsmax (* _alilioninteriorrotationsmax -1.0)) _alpha) 0.0))
        (Variables|MeshTransfroms|SetAlilionBackRightRotations (Math|Rotator|MakeRotator 0.0 (Math|Float|Lerp (.pitch (Variables|MeshTransfroms|GetAlilionBackRightRotations)) (Math|Float|MapRangeClamped (Input|EnhancedActionValues|GetIA_Rotate) -1.0 1.0 (* _alilioninteriorrotationsmax_2 -1.0) _alilioninteriorrotationsmax_2) _alpha) 0.0))))))

(event Custom|CleanUpLockOn
  ;[0.08438 0.01298 0.01229] Clean Up the targets array
  (Default|CleanUpSquence (Variables|Default|GetBPC_LockOnComponet)))

(event Custom|LandControl
  (bind _returnvalue (Game|GetPlayerController 0))
  (bind _returnvalue_2 (Transformation|GetActorForwardVector))
  (bind _wheelrotationsidemax (Variables|MeshTransfroms|GetWheelRotationSideMax))
  (bind _moveforwardinterp (Variables|Default|GetMoveForwardInterp))
  (bind _targetthrusterspeed (Variables|Speed|GetTargetThrusterSpeed))
  (bind _returnvalue_3 (/ _targetthrusterspeed 5e+02))
  (bind _returnvalue_4 (* _returnvalue_2 _moveforwardinterp _returnvalue_3))
  (bind (_x _y) (Math|Vector|BreakVector _returnvalue_4))
  ;[0 1 0.9575] Move Forward
  (Utilities|FlowControl|Sequence
    (:then_0
      ;;[1 1 1] Slowly move plane across ground, with speed getting higher the longer move forward is held down. Z is zero=ed out since it should not move up and only on same plane
      (Transformation|AddActorWorldOffset (Math|Vector|MakeVector _x _y 0.0))
      ;;[1 1 1] If Moving fast enough on ground and space is pressed, the plane will go into flying mode. Lag is turned on for sping arm for smother fly controlls and small offset added to prevent crashing on ground immediately upon take off
      (if (and (> (Variables|Default|GetMoveForwardInterp) 0.7) (or (Game|Player|IsInputKeyDown _returnvalue "G") (Game|Player|IsInputKeyDown _returnvalue "Gamepad_LeftThumbstick")))
        (Variables|Default|SetFlying? true)
        (bind _output_get (Variables|/Script/Engine.SpringArmComponent|SetbUsePawnControlRotation (Variables|Default|GetSpringArm) false))
        (Variables|/Script/Engine.CameraComponent|SetbUsePawnControlRotation (Variables|Default|GetCamera) _output_get)
        (Transformation|AddActorWorldOffset "0.000000,0.000000,25.000000")))
    (:then_1
      ;;[1 1 1] Setting Wheel Rotation for side and forward directions
      (Variables|MeshTransfroms|SetWheelRotation (Math|Rotator|MakeRotator 0.0 (+ (.pitch (Transformation|GetSocketRotation (Variables|Default|GetMesh) "front_wheel_1_jnt")) (* (Variables|Default|GetMoveForwardInterp) -5e+02)) (Math|Interpolation|FInterpTo (.yaw (Variables|MeshTransfroms|GetWheelRotation)) (Math|Float|MapRangeClamped (Input|EnhancedActionValues|GetIA_Rotate) -1.0 1.0 (* _wheelrotationsidemax -1.0) _wheelrotationsidemax) (Utilities|Time|GetWorldDeltaSeconds) 0.4))))))

(event Custom|SetFixedCamera
  (Utilities|FlowControl|RetriggerableDelay 1.0)
  (Components|Timeline|SetPlayRate (Variables|Default|GetCameraTimeline) 0.5)
  (Variables|Default|SetUpdatingCamera true)
  (bind _resetcamerapitch (Timeline|CameraTimeline PlayFromStart)
    (:Update
      (Pawn|SetControlRotation (Pawn|GetController) (Math|Rotator|Lerp(Rotator) (Pawn|GetControlRotation :!class /Script/Engine.Pawn) (Transformation|GetActorRotation) _resetcamerapitch true)))
    (:Finished
      (bind _output_get (Variables|/Script/Engine.SpringArmComponent|SetbUsePawnControlRotation (Variables|Default|GetSpringArm) false))
      (Variables|/Script/Engine.CameraComponent|SetbUsePawnControlRotation (Variables|Default|GetCamera) _output_get)
      (Pawn|SetControlRotation (Pawn|GetController) (Transformation|GetActorRotation))
      (Variables|Default|SetUpdatingCamera false))))

(event Custom|RestIntFlaps
  ;[0 1 0.9575] Move Forward
  (bind _newtrack_0 (Timeline|ResetIntiriorFlaps_TL PlayFromStart)
    (:Finished
      (Variables|MeshTransfroms|SetAlilionInteriorRotations (Math|Rotator|MakeRotator 0.0 (Math|Float|Lerp (.pitch (Variables|MeshTransfroms|GetAlilionInteriorRotations)) 0.0 _newtrack_0) 0.0)))))

(event Custom|SetBombIndicator
  (bind _returnvalue (Transformation|GetActorLocation))
  (bind _returnvalue_2 (Transformation|GetActorForwardVector))
  (bind _maximumthrusterspeed (Variables|Speed|GetMaximumThrusterSpeed))
  (bind _returnvalue_3 (* _maximumthrusterspeed 2.0))
  (bind _returnvalue_4 (* _returnvalue_2 _returnvalue_3))
  (bind _returnvalue_5 (+ _returnvalue _returnvalue_4))
  (Utilities|FlowControl|Sequence
    (:then_0
      (Utilities|FlowControl|DoOnce false
        (:Completed
          (bind _returnvalue_6 (Game|SpawnActorfromClass :Class "/Game/ArcadeSim/Blueprints/BP_BombIndicater.BP_BombIndicater_C" :CollisionHandlingOverride "Undefined" :TransformScaleMethod "MultiplyWithRoot" :Instigator 0))
          (Variables|Default|SetBombIndRef _returnvalue_6))))
    (:then_1
      (Variables|Default|GetBombIndRef
        (:then
          (bind _outhit (Collision|LineTraceByChannel _returnvalue_5 (+ _returnvalue_5 (* (Math|Vector|GetUpVector "0, 0, 0") -5e+04)) "TraceTypeQuery1" false 0 "ForDuration" true "(R=1.000000,G=0.000000,B=0.000000,A=1.000000)" "(R=0.000000,G=1.000000,B=0.000000,A=1.000000)" 1.0)))
        (:else)))))

(event Input|EnhancedActionEvents|EnhancedInputActionIA_MoveForward
  (params (ActionValue :type Float%20%28double-precision%29) (ElapsedSeconds :type Float%20%28double-precision%29) (TriggeredSeconds :type Float%20%28double-precision%29) (InputAction :type Input%20Action%20Object%20Reference :default "/Game/ArcadeSim/Inputs/Actions/Movement/IA_MoveForward.IA_MoveForward"))
  ;[0 1 0.9575] Move Forward
  ;;[1 1 1] If fly, then move forward inputs should increase/decrease flight speed. If not then it will add movement on floor using offset
  (:Triggered
    (if (Variables|Default|GetFlying?)
      (CallFunction|PitchControl ActionValue)
      (else
        (CallFunction|LandControl))))
  (:Completed
    (CallFunction|RestIntFlaps)))

(event Input|EnhancedActionEvents|EnhancedInputActionIA_Rotate
  (params (ActionValue :type Float%20%28double-precision%29) (ElapsedSeconds :type Float%20%28double-precision%29) (TriggeredSeconds :type Float%20%28double-precision%29) (InputAction :type Input%20Action%20Object%20Reference :default "/Game/ArcadeSim/Inputs/Actions/Movement/IA_Rotate.IA_Rotate"))
  ;[0 1 0.9575] Move right input. if not flying then move on ground if moving forward as well. The if not then inputs will no rotate the plane
  (:Triggered
    (Variables|PlaneRotation|SetRotateAV ActionValue)
    (if (Variables|Default|GetFlying?)
      (bind _output_get (Variables|PlaneRotation|SetFlightRoll (Math|Interpolation|FInterpTo (stale _output_get) ActionValue (Utilities|Time|GetWorldDeltaSeconds) 1e+01)))
      (Transformation|AddActorLocalRotation (Math|Rotator|MakeRotator (* _output_get (Utilities|Time|GetWorldDeltaSeconds) 9e+01) 0.0 0.0) false false)
      (CallFunction|AililreonRotate)
      (else
        ;;[1 1 1] Can only move right/left on ground if moving forward
        (if (> (Input|EnhancedActionValues|GetIA_MoveForward) 0.0)
          (Class|Actor|AddActorWorldRotation (Math|Rotator|MakeRotator 0.0 0.0 (* ActionValue (Utilities|Time|GetWorldDeltaSeconds) 1.2)))))))
  (:Completed
    (Variables|PlaneRotation|SetRotateAV 0.0)
    (CallFunction|AililreonRotate)))

(event Input|EnhancedActionEvents|EnhancedInputActionIA_SwicthSpecial3
  (params (ActionValue :type Boolean) (ElapsedSeconds :type Float%20%28double-precision%29) (TriggeredSeconds :type Float%20%28double-precision%29) (InputAction :type Input%20Action%20Object%20Reference :default "/Game/ArcadeSim/Inputs/Actions/IA_SwicthSpecial3.IA_SwicthSpecial3"))
  (:Started
    (Default|CallOnSwitchSpecial3)))

(event Input|EnhancedActionEvents|EnhancedInputActionIA_SwicthSpecial4
  (params (ActionValue :type Boolean) (ElapsedSeconds :type Float%20%28double-precision%29) (TriggeredSeconds :type Float%20%28double-precision%29) (InputAction :type Input%20Action%20Object%20Reference :default "/Game/ArcadeSim/Inputs/Actions/IA_SwicthSpecial4.IA_SwicthSpecial4"))
  (:Started
    (Default|CallOnSwitchSpecial4)))

(event Input|EnhancedActionEvents|EnhancedInputActionIA_LookUp
  (params (ActionValue :type Float%20%28double-precision%29) (ElapsedSeconds :type Float%20%28double-precision%29) (TriggeredSeconds :type Float%20%28double-precision%29) (InputAction :type Input%20Action%20Object%20Reference :default "/Game/ArcadeSim/Inputs/Actions/Movement/IA_LookUp.IA_LookUp"))
  ;[0 1 0.9575] Look up input. If not flying add camera rotation. If not then add rotation to plane and since spring arm is attached it will automatcally adjust camera behind plane
  (:Triggered
    (if (Variables|Default|GetFlying?)
      (if (not (Variables|Default|GetUpdatingCamera))
        (bind _output_get (Variables|/Script/Engine.SpringArmComponent|SetbUsePawnControlRotation (Variables|Default|GetSpringArm) true))
        (Variables|/Script/Engine.CameraComponent|SetbUsePawnControlRotation (Variables|Default|GetCamera) _output_get)
        (Pawn|Input|AddControllerPitchInput (* (* ActionValue (Math|Float|SelectFloat -1.0 1.0 (Variables|Default|GetInvertVerticalFlight?))) (Variables|Default|GetCameraSens)) :!label _label))
      (else
        (goto _label))))
  (:Completed
    (if (Variables|Default|GetFlying?)
      (CallFunction|SetFixedCamera))))

(event Input|EnhancedActionEvents|EnhancedInputActionIA_TurnRight
  (params (ActionValue :type Float%20%28double-precision%29) (ElapsedSeconds :type Float%20%28double-precision%29) (TriggeredSeconds :type Float%20%28double-precision%29) (InputAction :type Input%20Action%20Object%20Reference :default "/Game/ArcadeSim/Inputs/Actions/Movement/IA_TurnRight.IA_TurnRight"))
  ;[0 1 0.9575] Look up input. If not flying add camera rotation. If not then add rotation to plane and since spring arm is attached it will automatcally adjust camera behind plane
  (:Triggered
    (if (Variables|Default|GetFlying?)
      (if (not (Variables|Default|GetUpdatingCamera))
        (bind _output_get (Variables|/Script/Engine.SpringArmComponent|SetbUsePawnControlRotation (Variables|Default|GetSpringArm) true))
        (Variables|/Script/Engine.CameraComponent|SetbUsePawnControlRotation (Variables|Default|GetCamera) _output_get)
        (Pawn|Input|AddControllerYawInput (* ActionValue (Variables|Default|GetCameraSens)) :!label _label))
      (else
        (goto _label))))
  (:Completed
    (if (Variables|Default|GetFlying?)
      (CallFunction|SetFixedCamera))))

(event Input|EnhancedActionEvents|EnhancedInputActionIA_Fire
  (params (ActionValue :type Boolean) (ElapsedSeconds :type Float%20%28double-precision%29) (TriggeredSeconds :type Float%20%28double-precision%29) (InputAction :type Input%20Action%20Object%20Reference :default "/Game/ArcadeSim/Inputs/Actions/IA_Fire.IA_Fire"))
  ;[0 1 0.9575] Fire Gun
  (Default|CallOnGunShoot (Variables|Speed|GetCurrentThrusterSpeed) (Transformation|GetWorldLocation (Variables|Default|GetGunSocket))))

(event Input|EnhancedActionEvents|EnhancedInputActionIA_FireSpecial
  (params (ActionValue :type Boolean) (ElapsedSeconds :type Float%20%28double-precision%29) (TriggeredSeconds :type Float%20%28double-precision%29) (InputAction :type Input%20Action%20Object%20Reference :default "/Game/ArcadeSim/Inputs/Actions/IA_FireSpecial.IA_FireSpecial"))
  (bind _bpc_lockoncomponet (Variables|Default|GetBPC_LockOnComponet))
  ;[0 1 0.9575] Fire Special
  (:Started
    (if (Variables|/Game/ArcadeSim/Blueprints/BPC_LockOnComponet.BPC_LockOnComponet_C|GetLockedOn? _bpc_lockoncomponet)
      _
      (else
        _))
    (Default|CallOnMissleShoot (Variables|/Game/ArcadeSim/Blueprints/BPC_LockOnComponet.BPC_LockOnComponet_C|GetCloestTarget _bpc_lockoncomponet))))

(event Input|EnhancedActionEvents|EnhancedInputActionIA_LockOn
  (params (ActionValue :type Boolean) (ElapsedSeconds :type Float%20%28double-precision%29) (TriggeredSeconds :type Float%20%28double-precision%29) (InputAction :type Input%20Action%20Object%20Reference :default "/Game/ArcadeSim/Inputs/Actions/IA_LockOn.IA_LockOn"))
  ;[0 1 0.9575] Lock On To Cloest Target
  (:Started
    (Default|GrabClosestTarget (Variables|Default|GetBPC_LockOnComponet))))

(event Input|EnhancedActionEvents|EnhancedInputActionIA_IncreaseThrust
  (params (ActionValue :type Float%20%28double-precision%29) (ElapsedSeconds :type Float%20%28double-precision%29) (TriggeredSeconds :type Float%20%28double-precision%29) (InputAction :type Input%20Action%20Object%20Reference :default "/Game/ArcadeSim/Inputs/Actions/IA_IncreaseThrust.IA_IncreaseThrust"))
  ;[0 1 0.9575] Move Forward
  ;;[1 1 1] Increase/Decrease thrust
  (if (Variables|Default|GetFlying?)
    (Variables|Speed|SetTargetThrusterSpeed (Math|Float|Clamp(Float) (+ (* ActionValue (Utilities|Time|GetWorldDeltaSeconds) 2.5e+03) (Variables|Speed|GetTargetThrusterSpeed)) (Variables|Speed|GetMininumThrusterSpeed) (Variables|Speed|GetMaximumThrusterSpeed)))))

(event Input|EnhancedActionEvents|EnhancedInputActionIA_SwicthSpecial1
  (params (ActionValue :type Boolean) (ElapsedSeconds :type Float%20%28double-precision%29) (TriggeredSeconds :type Float%20%28double-precision%29) (InputAction :type Input%20Action%20Object%20Reference :default "/Game/ArcadeSim/Inputs/Actions/IA_SwicthSpecial1.IA_SwicthSpecial1"))
  (:Started
    (Default|CallOnSwitchSpecial1)))

(event Input|EnhancedActionEvents|EnhancedInputActionIA_SwicthSpecial2
  (params (ActionValue :type Boolean) (ElapsedSeconds :type Float%20%28double-precision%29) (TriggeredSeconds :type Float%20%28double-precision%29) (InputAction :type Input%20Action%20Object%20Reference :default "/Game/ArcadeSim/Inputs/Actions/IA_SwicthSpecial2.IA_SwicthSpecial2"))
  (:Started
    (Default|CallOnSwitchSpecial2)))

(event EventPassInputs
  (params (MaxLockOnTarget :type Integer))
  ;[0 1 0.9575] Lock On To Cloest Target
  (Variables|/Game/ArcadeSim/Blueprints/BPC_LockOnComponet.BPC_LockOnComponet_C|SetTargetAmount (Variables|Default|GetBPC_LockOnComponet) MaxLockOnTarget))

(event EventBeginPlay
  ;[0 0 0] Event BeginPlay
  (bind _asplayer_controller (Utilities|Casting|CastToPlayerController (Pawn|GetController)))
  (Utilities|IsValid (PlayerController|LocalPlayerSubsystems|GetEnhancedInputLocalPlayerSubsystem _asplayer_controller)
    (:Is%20Valid
      (Input|AddMappingContext (PlayerController|LocalPlayerSubsystems|GetEnhancedInputLocalPlayerSubsystem _asplayer_controller) "/Game/ArcadeSim/Inputs/Default_IMC.Default_IMC" 0 "(bIgnoreAllPressedKeysUntilRelease=True,bForceImmediately=False,bNotifyUserSettings=False)")
      (Utilities|FlowControl|Sequence
        (:then_0
          ;;[1 1 1] When Plane Take Off, It Should Fly At The Minimum Set Speed
          (Variables|Speed|SetTargetThrusterSpeed (Variables|Speed|GetMaximumThrusterSpeed))
          ;;[1 1 1] Setting offset for landing trace
          (Variables|Default|SetStarZOffset (Variables|Default|GetPlaneZOffset)))
        (:then_1
          ;;[1 1 1] Set Scale of exhaust particles to 0 as it should become more intense with speed
          (Transformation|SetRelativeScale3D (Variables|Default|GetLeftExhaust) "0, 0, 0"))
        (:then_2
          ;;[1 1 1] Attach Special To Player
          (Default|CallOnAttachMissle))))))

(event EventTick
  (params (DeltaSeconds :type Float%20%28single-precision%29))
  (bind _leftexhaust (Variables|Default|GetLeftExhaust))
  (bind _currentthrusterspeed (Variables|Speed|GetCurrentThrusterSpeed))
  (bind _maximumthrusterspeed (Variables|Speed|GetMaximumThrusterSpeed))
  (bind _returnvalue (Math|Float|NormalizetoRange _currentthrusterspeed 0.0 _maximumthrusterspeed))
  ;[0 0 0] Event Tick
  (Utilities|FlowControl|Sequence
    (:then_0
      ;;[1 1 1] For Grounded Movement. Intrep value set to low value as jet should speed up very gradually when on ground
      (bind _output_get (Variables|Default|SetMoveForwardInterp (Math|Float|Clamp(Float) (Math|Interpolation|FInterpTo (stale _output_get) (Input|EnhancedActionValues|GetIA_MoveForward) (Utilities|Time|GetWorldDeltaSeconds) 0.2))))
      ;[1 1 1] Set exhaust particle scale relative to speed. 0 If not flying but interp speed is low so if landing it while take a while for the aprticles fade to zero scale
      (Transformation|SetRelativeScale3D _leftexhaust (Math|Interpolation|VInterpTo (Variables|/Script/Engine.SceneComponent|GetRelativeScale3D _leftexhaust) (Math|Vector|SelectVector (Math|Vector|MakeVector _returnvalue _returnvalue _returnvalue) "0, 0, 0" (Variables|Default|GetFlying?)) (Utilities|Time|GetWorldDeltaSeconds) (Math|Float|SelectFloat 4.0 0.5 (Variables|Default|GetFlying?)))))
    (:then_1
      ;;[1 1 1] Is Flying
      (if (Variables|Default|GetFlying?)
        (CallFunction|AddFlightMovement)
        (CallFunction|LandingTrace "ForOneFrame" (Variables|Default|GetStarZOffset))
        (CallFunction|SetCameraLag)))))

(event Input|KeyboardEvents|DebugKeyT
  (params (Key :type Key%20Structure :default "None") (ActionValue :type Input%20Action%20Value%20Structure)))

(fn ConstructionScript)

(fn AddFlightMovement
  (bind _returnvalue (Utilities|Time|GetWorldDeltaSeconds))
  ;[1 1 1] Set flight Speed
  (bind _output_get (Variables|Speed|SetCurrentThrusterSpeed (Math|Interpolation|FInterpTo (stale _output_get) (Variables|Speed|GetTargetThrusterSpeed) _returnvalue 8.0)))
  ;[1 1 1] Add movement in forward direction to plane
  (Transformation|AddActorWorldOffset (* (Math|Vector|GetForwardVector (Variables|Default|GetMesh)) (* _output_get _returnvalue)) true))

(fn LandingTrace
  (params (Debug :type EDrawDebugTrace%20Enum :default "None") (Spawned%20Z%20Offset :type Float%20%28double-precision%29))
  (bind _returnvalue (Transformation|GetActorLocation))
  ;[1 1 1] Do line trace from plane center to postion under the wheel
  (bind (_outhit _returnvalue_2) (Collision|LineTraceByChannel _returnvalue (- _returnvalue (Math|Vector|MakeVector 0.0 0.0 Spawned%20Z%20Offset)) "TraceTypeQuery1" false (Utilities|Array|MakeArray self) Debug))
  ;[1 1 1] Can only land if speed is low enough(controlled by holding move forward or backward)
  (if _returnvalue_2
    (if (< (Math|Float|MapRangeClamped (Variables|Speed|GetTargetThrusterSpeed) (Variables|Speed|GetMininumThrusterSpeed) (Variables|Speed|GetMaximumThrusterSpeed) 0.0 1.0) 0.5)
      ;[1 1 1] Align plane with floor(using custom variables instead of normals). Rotation is only retained a yaw. Location include of wheels offset
      (Variables|Default|SetFlying? false)
      (Transformation|SetActorRelativeTransform (Math|Transform|MakeTransform (Math|Interpolation|VInterpTo (Transformation|GetActorLocation) (+ (.TraceEnd (Collision|BreakHitResult _outhit)) (Math|Vector|MakeVector 0.0 0.0 Spawned%20Z%20Offset)) (Utilities|Time|GetWorldDeltaSeconds) 3.0) (Math|Rotator|MakeRotator 0.0 0.0 (.yaw (Transformation|GetActorRotation))) "1.000000,1.000000,1.000000") false false)
      ;[1 1 1] Set variables
      (Variables|/Script/Engine.SpringArmComponent|SetbUsePawnControlRotation (Variables|Default|GetSpringArm) true)
      (Variables|Default|SetMoveForwardInterp 1.0))))

(fn SetCameraLag
  (bind _springarm (Variables|Default|GetSpringArm))
  (bind _flying_ (Variables|Default|GetFlying?))
  (bind _returnvalue (Math|Float|SelectFloat 1e+01 1e+03 _flying_))
  ;[1 1 1] If not flying the lag should be hign enough to not be recongnisable since it is still recuired for smooth camera return when landing
  (Variables|/Script/Engine.SpringArmComponent|SetCameraLagSpeed _springarm _returnvalue)
  (Variables|/Script/Engine.SpringArmComponent|SetCameraRotationLagSpeed _springarm _returnvalue))

(fn PitchControl
  (params (Action%20Value :type Float%20%28double-precision%29))
  (bind _returnvalue (Utilities|Time|GetWorldDeltaSeconds))
  (bind _alilioninteriorrotationsmax (Variables|MeshTransfroms|GetAlilionInteriorRotationsMax))
  (bind _output_get (Variables|PlaneRotation|SetFlightPitch (Math|Interpolation|FInterpTo (Variables|PlaneRotation|GetFlightPitch) (* Action%20Value (Math|Float|SelectFloat -1.0 1.0 (Variables|Default|GetInvertVerticalFlight?))) _returnvalue 1e+01)))
  (Transformation|AddActorLocalRotation (Math|Rotator|MakeRotator 0.0 (* _output_get _returnvalue (Variables|PlaneRotation|GetFlightTurnRate)) 0.0) false false)
  (Variables|MeshTransfroms|SetAlilionInteriorRotations (Math|Rotator|MakeRotator 0.0 (Math|Float|MapRangeClamped (Variables|PlaneRotation|GetFlightPitch) -1.0 1.0 _alilioninteriorrotationsmax (* _alilioninteriorrotationsmax -1.0)) 0.0)))