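; Lock-on component that finds "Target"-tagged actors near its owner and picks up to TargetAmount of them to lock onto.
; Tick adds in-range actors to PossibleTargets, drawing debug spheres that distinguish candidates from picked targets.
; GrabClosestTarget builds a chain through a distance-loop macro, searching nearest to the owner first, then to each previous pick, and sets LockedOn.
; CleanUpSquence prunes invalid actors and clears candidates; "Old Code" is an unused single-target version.
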(event `MarkTargets`
  ;[0.08438 0.01298 0.01229] Check to see if the arre doesnt allready contain the target actor and the current actor then add current actor to possible targets
  (`KismetSystemLibrary.DrawDebugSphere` (`Actor.K2_GetActorLocation` (`self.CurrentActor`)) 200.0 12 (struct :`G` 1.0 :`B` 0.118767 :`A` 1.0))
  (if (not (`KismetArrayLibrary.Array_Contains` (`self.PossibleTargets`) (`self.CurrentActor`)))
    (`KismetArrayLibrary.Array_Add` (`self.PossibleTargets`) (`self.CurrentActor`))))

(event `self.ReceiveBeginPlay`
  ;[0 0 0] Event BeginPlay, set delay for 1 second and then get all acotes with the tag Targets and set them to an array
  (`KismetSystemLibrary.Delay` 1.0)
  (bind _outactors (`GameplayStatics.GetAllActorsWithTag` "Target"))
  (set `self.TargetActors` _outactors)
  (set `self.HasTargets?` true))

(event `CheckTargetDistance`
  ;[0.08438 0.01298 0.01229] CheckTargetDistance by starting a for each loop check the disntace from player to the target
  (bind (_array_element _distance) (`self.GetDistanceFromArray` (`self.TargetActors`) (`self.GetOwner`))
    (:`Exit`
      (set `self.CurrentActor` _array_element)
      (if (<= _distance (`self.TargetDistance`))
        (if (`KismetArrayLibrary.Array_IsNotEmpty` (`self.CloestTargetA`))
          (if (`KismetArrayLibrary.Array_Contains` (`self.CloestTargetA`) (`self.CurrentActor`))
            (`self.MarkCloestTarget` (`self.CurrentActor`))
            (else
              (`self.MarkTargets`)))
          (else
            (`self.MarkTargets`)))))))

(event `MarkCloestTarget`
  (params (`Target To Mark` :type "Actor Object Reference"))
  ;[0.08438 0.01298 0.01229] MarkCloestTarget
  (`/Engine/EditorBlueprintResources/StandardMacros.IsValid` `Target To Mark`
    (:`Is Valid`
      (`KismetSystemLibrary.DrawDebugSphere` (`Actor.K2_GetActorLocation` `Target To Mark`) 200.0 12 (struct :`R` 1.0 :`G` 0.054508 :`A` 1.0)))))

(event `self.ReceiveTick`
  (params (DeltaSeconds :type "Float (single-precision)"))
  ;[0 0 0] EventTick
  (if (`self.HasTargets?`)
    (`self.CheckTargetDistance`)))

(event `GrabClosestTarget`
  ;[0.08438 0.01298 0.01229] GrabCloestTarget Start a for loop by Target Amount variable and sumtract the amout by one so for loop starts at 0 first time it goes set cloest dstance to -1 and ceck to cloest target to the player and store first index. The on next time set closet distance to -1 and set to next index and then compare last cloest target and check to see if it's valit and set it do ditance to and compare the distance to last cloest target and set to the array index.
  (for _index (range (`self.TargetAmount`))
    (set `self.CloestDistance` -1.0)
    (if (== _index 0)
      (set `self.DistanceTo` (`self.GetOwner`))
      (else
        (bind _output (`|GetArrayItem` (`self.CloestTargetA`) (- _index 1)))
        (`/Engine/EditorBlueprintResources/StandardMacros.IsValid` _output
          (:`Is Valid`
            (bind _output_get (set `self.DistanceTo` _output))))))
    (bind (_array_element _distance) (`self.GetDistanceFromArray` (`self.PossibleTargets`) _output_get)
      (:`Exit`
        (if (< (`self.CloestDistance`) 0.0)
          (`KismetArrayLibrary.Array_Add` (`self.CloestTargetA`) _array_element)
          (set `self.CloestDistance` _distance)
          (elif (< _distance (`self.CloestDistance`))
            (`KismetArrayLibrary.Array_Set` (`self.CloestTargetA`) _index _array_element)
            (set `self.CloestDistance` _distance))))))
  (if (`KismetArrayLibrary.Array_IsNotEmpty` (`self.CloestTargetA`))
    (set `self.LockedOn?` true)))

(event `CleanUp Squence`
  ;[0.08438 0.01298 0.01229] Go through array and check if each elment is vaild and if it isn't remove it
  (set `self.HasTargets?` false)
  (for (_array_element _array_index) (`self.TargetActors`)
    (`/Engine/EditorBlueprintResources/StandardMacros.IsValid` _array_element
      (:`Is Not Valid`
        (`KismetArrayLibrary.Array_Remove` (`self.TargetActors`) _array_index))))
  (`KismetArrayLibrary.Array_Clear` (`self.PossibleTargets`))
  (set `self.HasTargets?` true))