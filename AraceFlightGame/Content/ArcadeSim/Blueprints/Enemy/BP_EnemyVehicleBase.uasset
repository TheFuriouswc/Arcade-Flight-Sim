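; Base enemy vehicle Blueprint that reacts to any damage by spawning a wreck actor and an explosion effect.
; It then calls a voiceline helper that plays a kill quip at the player pawn with a data-table-driven subtitle widget.
; Each quip check rolls a new random number, so all can miss and print "failed".
; The vehicle is destroyed from the helper's successful exit.
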(event `self.ReceiveAnyDamage`
  (params (Damage :type "Float (single-precision)") (DamageType :type "DamageType Object Reference") (InstigatedBy :type "Controller Object Reference") (DamageCauser :type "Actor Object Reference"))
  (bind _returnvalue (`KismetMathLibrary.RandomIntegerInRange` 1 4))
  (`|SpawnActorFromClass` "/Game/ArcadeSim/Blueprints/Enemy/BP_EnemyVehicleWreckBase.BP_EnemyVehicleWreckBase_C" (`KismetMathLibrary.MakeTransform` (`self.K2_GetActorLocation`) (`self.K2_GetActorRotation`)) "Undefined" "MultiplyWithRoot" null null)
  (`NiagaraFunctionLibrary.SpawnSystemAtLocation` "/Game/ArcadeSim/VFX/Particles/FXS_BOOM.FXS_BOOM" (`self.K2_GetActorLocation`) (`self.K2_GetActorRotation`) (`self.GetActorScale3D`))
  (if (== _returnvalue 1.0)
    (`self.SpawnSubtitles` "/Game/ArcadeSim/SoundEffects/Voicelines/Player/shack_.shack_" "/Game/ArcadeSim/Subtitles/Player/DTSub_PlayerKill3.DTSub_PlayerKill3")
    (`self.K2_DestroyActor` :!label _label)
    (elif (== _returnvalue 2.0)
      (`self.SpawnSubtitles` "/Game/ArcadeSim/SoundEffects/Voicelines/Player/goodeffectontarget.goodeffectontarget" "/Game/ArcadeSim/Subtitles/Player/DTSub_PlayerKill4.DTSub_PlayerKill4")
      (goto _label)
      (elif (== _returnvalue 3.0)
        (`self.SpawnSubtitles` "/Game/ArcadeSim/SoundEffects/Voicelines/Player/thatsoneforthereel.thatsoneforthereel" "/Game/ArcadeSim/Subtitles/Player/DTSub_PlayerKill5.DTSub_PlayerKill5")
        (goto _label)
        (elif (== _returnvalue 4.0)
          (`self.SpawnSubtitles` "/Game/ArcadeSim/SoundEffects/Voicelines/Player/hotdamn.hotdamn" "/Game/ArcadeSim/Subtitles/Player/DTSub_PlayerKill6.DTSub_PlayerKill6")
          (goto _label)
          (else
            (`KismetSystemLibrary.PrintString` "failed")))))))

(fn `UserConstructionScript`)