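; Example flying AI pawn in the enemy jets folder that repeatedly moves toward the location of player controller 0's actor.
; After a short random delay at BeginPlay, it sends BPFlyingAiPathfinding a ServerMoveTo slightly below that location.
; A self-calling event then re-targets the unoffset location after longer random delays, printing a debug string.
; The location is read from the controller itself, rather than its possessed pawn.
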(event `self.ReceiveBeginPlay`
  (bind (_returnvalue_x _returnvalue_y _returnvalue_z) (`KismetMathLibrary.BreakVector` (`self.K2_GetActorLocation` (`GameplayStatics.GetPlayerController` 0))))
  ;[1 1 1] Example Move To Target Location
  (`KismetSystemLibrary.Delay` (`KismetMathLibrary.RandomFloatInRange` 2.0 5.0))
  (`/Game/FlyingAIPathfinding/Blueprints/BP_FlyingAiPathfinding.Server_MoveTo` (`self.BP_FlyingAiPathfinding`) (`KismetMathLibrary.MakeVector` _returnvalue_x _returnvalue_y (+ _returnvalue_z -200.0)))
  (`self.Get Player location`))

(event `Get Player location`
  (`KismetSystemLibrary.Delay` (`KismetMathLibrary.RandomFloatInRange` 5.0 25.0))
  (`/Game/FlyingAIPathfinding/Blueprints/BP_FlyingAiPathfinding.Server_MoveTo` (`self.BP_FlyingAiPathfinding`) (`self.K2_GetActorLocation` (`GameplayStatics.GetPlayerController` 0)))
  (`self.Get Player location`)
  (`KismetSystemLibrary.PrintString` "Get Player Location"))

(fn `UserConstructionScript`)